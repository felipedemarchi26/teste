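; Player Blueprint for a furniture placement scene, letting the user spawn, drag, rotate and restyle furniture with keyboard and mouse.
; Number keys spawn a Furniture actor at a preset height and assign its mesh, scale and rotation.
; Cursor traces select furniture: left-drag follows the cursor on Tick keeping Z, right-drag yaws it with MouseY.
; Up and Down arrows cycle materials on the last spawned or left-clicked piece.
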(event `self.ReceiveTick`
  (params (DeltaSeconds :type "Float (single-precision)"))
  (`self.MoveFurniture`))

(event `Key|One`
  (params (Key :type "Key Structure" :default "AnyKey"))
  ;[1 1 1] Eventos para adicionar os móveis na cena
  (:`Pressed`
    (bind _spawnedfurniture (`self.SpawnFurniture` 20.0))
    (`self.DefineFurniture` 1 _spawnedfurniture)))

(event `self.ReceiveBeginPlay`
  ;[1 1 1] Habilita o input no BeginPlay
  (`self.EnableInput` (`GameplayStatics.GetPlayerController` 0)))

(event `Key|Two`
  (params (Key :type "Key Structure" :default "AnyKey"))
  ;[1 1 1] Eventos para adicionar os móveis na cena
  (:`Pressed`
    (bind _spawnedfurniture (`self.SpawnFurniture` 170.0))
    (`self.DefineFurniture` 2 _spawnedfurniture)))

(event `Key|Three`
  (params (Key :type "Key Structure" :default "AnyKey"))
  ;[1 1 1] Eventos para adicionar os móveis na cena
  (:`Pressed`
    (bind _spawnedfurniture (`self.SpawnFurniture` 660.0))
    (`self.DefineFurniture` 3 _spawnedfurniture)))

(event `Key|Up`
  (params (Key :type "Key Structure" :default "AnyKey"))
  (bind _furnitureselectedmaterial (`self.FurnitureSelectedMaterial`))
  ;[1 1 1] Altera o material ao pressionar a seta para cima
  (:`Pressed`
    (`/Game/Blueprints/Furniture.ChangeIndexUp` _furnitureselectedmaterial)
    (`/Game/Blueprints/Furniture.ChangeMaterial` _furnitureselectedmaterial)))

(event `Key|Four`
  (params (Key :type "Key Structure" :default "AnyKey"))
  ;[1 1 1] Eventos para adicionar os móveis na cena
  (:`Pressed`
    (bind _spawnedfurniture (`self.SpawnFurniture` 0.0))
    (`self.DefineFurniture` 4 _spawnedfurniture)))

(event `Key|Five`
  (params (Key :type "Key Structure" :default "AnyKey"))
  ;[1 1 1] Eventos para adicionar os móveis na cena
  (:`Pressed`
    (bind _spawnedfurniture (`self.SpawnFurniture` 130.0))
    (`self.DefineFurniture` 5 _spawnedfurniture)))

(event `Key|Down`
  (params (Key :type "Key Structure" :default "AnyKey"))
  (bind _furnitureselectedmaterial (`self.FurnitureSelectedMaterial`))
  ;[1 1 1] Altera o material ao pressionar a seta para baixo
  (:`Pressed`
    (`/Game/Blueprints/Furniture.ChangeIndexDown` _furnitureselectedmaterial)
    (`/Game/Blueprints/Furniture.ChangeMaterial` _furnitureselectedmaterial)))

(event `Key|Six`
  (params (Key :type "Key Structure" :default "AnyKey"))
  ;[1 1 1] Eventos para adicionar os móveis na cena
  (:`Pressed`
    (bind _spawnedfurniture (`self.SpawnFurniture` 50.0))
    (`self.DefineFurniture` 6 _spawnedfurniture)))

(event `Key|Seven`
  (params (Key :type "Key Structure" :default "AnyKey"))
  ;[1 1 1] Eventos para adicionar os móveis na cena
  (:`Pressed`
    (bind _spawnedfurniture (`self.SpawnFurniture` 0.0))
    (`self.DefineFurniture` 7 _spawnedfurniture)))

(event `InputAxisKey|MouseY`
  (params (AxisValue :type "Float (single-precision)"))
  ;[1 1 1] Rotaciona o móvel
  (`self.RotateFurniture` AxisValue))

(event `Key|Eight`
  (params (Key :type "Key Structure" :default "AnyKey"))
  ;[1 1 1] Eventos para adicionar os móveis na cena
  (:`Pressed`
    (bind _spawnedfurniture (`self.SpawnFurniture` 0.0))
    (`self.DefineFurniture` 8 _spawnedfurniture)))

(event `Key|Nine`
  (params (Key :type "Key Structure" :default "AnyKey"))
  ;[1 1 1] Eventos para adicionar os móveis na cena
  (:`Pressed`
    (bind _spawnedfurniture (`self.SpawnFurniture` 40.0))
    (`self.DefineFurniture` 9 _spawnedfurniture)))

(event `Key|LeftMouseButton`
  (params (Key :type "Key Structure" :default "AnyKey"))
  (bind (_bblockinghit _binitialoverlap _time _location _impactpoint _normal _impactnormal _physmat _hitactor) (`GameplayStatics.BreakHitResult` (`PlayerController.GetHitResultUnderCursorForObjects` (`GameplayStatics.GetPlayerController` 0) (`|MakeArray` "ObjectTypeQuery1" :!type "EObjectTypeQuery Enum") true)))
  ;[1 1 1] Gerencia se o botão esquerdo do mouse está pressionado e se clicou sobre algum móvel para permitir a sua movimentação
  (:`Pressed`
    (`/Engine/EditorBlueprintResources/StandardMacros.IsValid` _hitactor
      (:`Is Valid`
        (bind _asfurniture (cast `/Game/Blueprints/Furniture` _hitactor))
        (set `self.FurnitureSelected` _asfurniture)
        (set `self.FurnitureSelectedMaterial` _asfurniture)
        (set `self.LeftButon` true)
        (set `self.RightButton` false))))
  (:`Released`
    (set `self.LeftButon` false)
    (set `self.FurnitureSelected` null)))

(event `Key|RightMouseButton`
  (params (Key :type "Key Structure" :default "AnyKey"))
  (bind (_bblockinghit _binitialoverlap _time _location _impactpoint _normal _impactnormal _physmat _hitactor) (`GameplayStatics.BreakHitResult` (`PlayerController.GetHitResultUnderCursorForObjects` (`GameplayStatics.GetPlayerController` 0) (`|MakeArray` "ObjectTypeQuery1" :!type "EObjectTypeQuery Enum") true)))
  ;[1 1 1] Gerencia se o botão direito do mouse está pressionado e se foi clicado sobre um móvel para a sua rotação
  (:`Pressed`
    (`/Engine/EditorBlueprintResources/StandardMacros.IsValid` _hitactor
      (:`Is Valid`
        (bind _asfurniture (cast `/Game/Blueprints/Furniture` _hitactor))
        (set `self.FurnitureSelected` _asfurniture)
        (set `self.RightButton` true)
        (set `self.LeftButon` false))))
  (:`Released`
    (set `self.RightButton` false)
    (set `self.FurnitureSelected` null)))

(fn `DefineFurniture`
  (params (KeyPressed :type Integer) (Furniture :type "/Game/Blueprints/Furniture Object Reference"))
  (bind _staticmesh (`/Game/Blueprints/Furniture.StaticMesh` Furniture))
  (set `self.FurnitureSelectedMaterial` Furniture)
  (switch `int` KeyPressed
    (:`1`
      (`StaticMeshComponent.SetStaticMesh` _staticmesh "/Game/Furnitures/Desk/desk.desk"))
    (:`2`
      (`StaticMeshComponent.SetStaticMesh` _staticmesh "/Game/Furnitures/Dresser/Dresser_Dresser.Dresser_Dresser")
      (`SceneComponent.SetWorldScale3D` _staticmesh (1.5 1.5 1.5))
      (`SceneComponent.K2_SetWorldRotation` _staticmesh (struct :`Yaw` 180.0) false false))
    (:`3`
      (`StaticMeshComponent.SetStaticMesh` _staticmesh "/Game/Furnitures/Rack/Rack.Rack")
      (`SceneComponent.SetWorldScale3D` _staticmesh (10.0 10.0 10.0))
      (`SceneComponent.K2_SetWorldRotation` _staticmesh (struct :`Yaw` -90.0) false false))
    (:`4`
      (`StaticMeshComponent.SetStaticMesh` _staticmesh "/Game/Furnitures/Sofa2/Sofa_FREE_FBX.Sofa_FREE_FBX")
      (`SceneComponent.SetWorldScale3D` _staticmesh (7.0 7.0 7.0))
      (`SceneComponent.K2_SetWorldRotation` _staticmesh (struct :`Yaw` 90.0) false false))
    (:`5`
      (`StaticMeshComponent.SetStaticMesh` _staticmesh "/Game/Furnitures/Table/table.table")
      (`SceneComponent.SetWorldScale3D` _staticmesh (150.0 150.0 150.0)))
    (:`6`
      (`StaticMeshComponent.SetStaticMesh` _staticmesh "/Game/Furnitures/WoodTable/tableBake_Table_body_000.tableBake_Table_body_000")
      (`SceneComponent.K2_SetWorldRotation` _staticmesh (struct :`Yaw` 90.0) false false))
    (:`7`
      (`StaticMeshComponent.SetStaticMesh` _staticmesh "/Game/Furnitures/Dresser2/Table_polySurface21.Table_polySurface21")
      (`SceneComponent.SetWorldScale3D` _staticmesh (100.0 100.0 100.0))
      (`SceneComponent.K2_SetWorldRotation` _staticmesh (struct :`Yaw` 90.0) false false))
    (:`8`
      (`StaticMeshComponent.SetStaticMesh` _staticmesh "/Game/Furnitures/Table2/Table_polySurface20.Table_polySurface20")
      (`SceneComponent.SetWorldScale3D` _staticmesh (100.0 100.0 100.0))
      (`SceneComponent.K2_SetWorldRotation` _staticmesh (struct :`Yaw` 90.0) false false))
    (:`9`
      (`StaticMeshComponent.SetStaticMesh` _staticmesh "/Game/Furnitures/WoodTable2/modernTable_Table.modernTable_Table")
      (`SceneComponent.K2_SetWorldRotation` _staticmesh (struct :`Yaw` -90.0) false false))))

(fn `MoveFurniture`
  (bind (_returnvalue_x _returnvalue_y _returnvalue_z) (`KismetMathLibrary.BreakVector` (`self.K2_GetActorLocation` (`self.FurnitureSelected`))))
  ;[1 1 1] Verifica se o botão esquerdo do mouse foi pressionado
  (if (`self.LeftButon`)
    ;[1 1 1] Verifica se existe algum móvel selecionado
    (`/Engine/EditorBlueprintResources/StandardMacros.IsValid` (`self.FurnitureSelected`)
      (:`Is Valid`
        ;[1 1 1] Define a nova localização do móvel com base no ponteiro do mouse
        (`self.K2_SetActorLocation` (`self.FurnitureSelected`) (`KismetMathLibrary.MakeVector` (.x (`.Location` (`GameplayStatics.BreakHitResult` (`PlayerController.GetHitResultUnderCursorByChannel` (`GameplayStatics.GetPlayerController` 0) "TraceTypeQuery1" true)))) (.y (`.Location` (`GameplayStatics.BreakHitResult` (`PlayerController.GetHitResultUnderCursorByChannel` (`GameplayStatics.GetPlayerController` 0) "TraceTypeQuery1" true)))) _returnvalue_z) false false)))))

(fn `RotateFurniture`
  (params (YValue :type "Float (double-precision)"))
  (bind _furnitureselected (`self.FurnitureSelected`))
  (`/Engine/EditorBlueprintResources/StandardMacros.IsValid` (`self.FurnitureSelected`)
    (:`Is Valid`
      (if (`self.RightButton`)
        (`self.K2_SetActorRotation` _furnitureselected (`KismetMathLibrary.MakeRotator` (.roll (`self.K2_GetActorRotation` _furnitureselected)) (.pitch (`self.K2_GetActorRotation` _furnitureselected)) (+ (.yaw (`self.K2_GetActorRotation` _furnitureselected)) (* YValue -4.0))) false)))))

(fn `SpawnFurniture`
  (params (ZValue :type "Float (double-precision)"))
  (returns (SpawnedFurniture :type "/Game/Blueprints/Furniture Object Reference"))
  (bind _returnvalue (`|SpawnActorFromClass` "/Game/Blueprints/Furniture.Furniture_C" (`KismetMathLibrary.MakeTransform` (`KismetMathLibrary.MakeVector` 0.0 0.0 ZValue)) "Undefined" "OverrideRootScale"))
  (return _returnvalue))

(fn `UserConstructionScript`)