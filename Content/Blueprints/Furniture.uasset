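; Furniture actor whose static mesh can switch between four wood and cork materials.
; BeginPlay resets the material index to the first option, bamboo, and applies it to the first material slot only.
; ChangeIndexUp and ChangeIndexDown step the index with wraparound but do not update the mesh.
; ChangeMaterial, a separate function, applies the indexed material to every slot; nothing in this Blueprint calls these three functions.
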(event `self.ReceiveBeginPlay`
  (set `self.IndexMaterial` 0)
  (`PrimitiveComponent.SetMaterial` (`self.StaticMesh`) 0 "/Game/Materials/Bamboo/bamboo-wood-semigloss-albedo_Mat.bamboo-wood-semigloss-albedo_Mat"))

(fn `ChangeIndexDown`
  (bind _indexmaterial (`self.IndexMaterial`))
  (if (== _indexmaterial 0)
    (set `self.IndexMaterial` 3)
    (else
      (set `self.IndexMaterial` (- _indexmaterial 1)))))

(fn `ChangeIndexUp`
  (bind _indexmaterial (`self.IndexMaterial`))
  (if (== _indexmaterial 3)
    (set `self.IndexMaterial` 0)
    (else
      (set `self.IndexMaterial` (+ _indexmaterial 1)))))

(fn `ChangeMaterial`
  (bind _staticmesh (`self.StaticMesh`))
  (for (_ _array_index) (`MeshComponent.GetMaterials` (`self.StaticMesh`))
    (switch `int` (`self.IndexMaterial`)
      (:`0`
        (`PrimitiveComponent.SetMaterial` _staticmesh _array_index "/Game/Materials/Bamboo/bamboo-wood-semigloss-albedo_Mat.bamboo-wood-semigloss-albedo_Mat"))
      (:`1`
        (`PrimitiveComponent.SetMaterial` _staticmesh _array_index "/Game/Materials/Corkboard/corkboard3b-albedo_Mat.corkboard3b-albedo_Mat"))
      (:`2`
        (`PrimitiveComponent.SetMaterial` _staticmesh _array_index "/Game/Materials/M_Wood_Oak.M_Wood_Oak"))
      (:`3`
        (`PrimitiveComponent.SetMaterial` _staticmesh _array_index "/Game/Materials/M_Wood_Pine.M_Wood_Pine")))))

(fn `UserConstructionScript`)